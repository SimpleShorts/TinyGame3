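; Player controller for the game-over screen, whose only working behaviour is quitting the game when Q is pressed.
; Possess, score and lives events are empty, and the interface functions for next level and persistent data return zeros.
; Disconnected leftover logic would create score, lives, end title and final score widgets, update them, and spawn a ball from the bat pawn, but never runs.
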(event EventPossess
  (params (PossessedPawn :type Pawn%20Object%20Reference))
  ;[1 1 1] On Possess
)

(event EventBPIScoreUpdate
  (params (Points :type Integer))
  ;[1 1 1] Update Score UI
)

(event EventBPILivesUpdate
  (params (LIves :type Integer))
  ;[1 1 1] Update Lives UI
)

(event Input|ActionEvents|InputActionInput-Positive
  (params (Key :type Key%20Structure :default "None"))
  ;[1 1 1] User Click to Spawn Ball
)

(event Input|KeyboardEvents|Q
  (params (Key :type Key%20Structure :default "None"))
  (:Pressed
    (Game|QuitGame 0 "Quit" false)))

(fn ConstructionScript)

(fn BPIRequestNextLevel
  (return 0))

(fn BPIRetrievePersistentData
  (return 0 0))