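; Player controller for the end screen of a bat-and-ball game, showing the title, final score, score and lives.
; Possessing a BP_Pawn_Bat creates the four UI widgets and adds them to the viewport.
; Interface events push score, after a short delay, to both score widgets and lives to the lives widget.
; Next-level and persistent-data functions are stubs returning zeros, and the ball-spawn logic is unconnected.
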(event EventBeginPlay)

(event EventPossess
  (params (PossessedPawn :type Pawn%20Object%20Reference))
  (bind _self self)
  ;[1 1 1] On Possess
  (bind _asbp_pawn_bat (Utilities|Casting|CastToBP_Pawn_Bat PossessedPawn)
    (:then
      (Variables|Default|SetAs%20BP%20Pawn%20Bat _asbp_pawn_bat)
      (bind _returnvalue (UserInterface|CreateWidget "/Game/Framework/UI/UI_Score.UI_Score_C" _self))
      (Variables|Default|SetDisplayed_Score _returnvalue)
      (bind _returnvalue_2 (UserInterface|CreateWidget "/Game/Framework/UI/UI_Lives.UI_Lives_C" _self))
      (Variables|Default|SetDisplayed_Lives _returnvalue_2)
      (UserInterface|Viewport|AddtoViewport (Variables|Default|GetDisplayed_Score) 0)
      (Development|PrintString "We loaded the BP Player Controller End SCrune" true true "(R=0.192026,G=0.000000,B=1.000000,A=1.000000)" 2e+01)
      (bind _returnvalue_3 (UserInterface|CreateWidget "/Game/Framework/UI/UI_EndTitle.UI_EndTitle_C"))
      (bind _output_get (Variables|Default|SetUI%20End%20Title _returnvalue_3))
      (UserInterface|Viewport|AddtoViewport _output_get 0)
      (bind _returnvalue_4 (UserInterface|CreateWidget "/Game/Framework/UI/UI_FinalScore.UI_FinalScore_C" self))
      (Variables|Default|SetDisplayed_Score2 _returnvalue_4)
      (UserInterface|Viewport|AddtoViewport (Variables|Default|GetDisplayed_Score2) 0))
    (:CastFailed
      (Development|PrintString "Oh shart, didn't cast"))))

(event EventBPIScoreUpdate
  (params (Points :type Integer))
  ;[1 1 1] Update Score UI
  (Utilities|FlowControl|Delay 0.1)
  (Default|UpdateScore (Variables|Default|GetDisplayed_Score) Points)
  (Default|UpdateScore (Variables|Default|GetDisplayed_Score2) Points)
  (Development|PrintString "Well we tried updating in both update scores..." true true "(R=0.000000,G=0.660000,B=1.000000,A=1.000000)" 1e+01))

(event EventBPILivesUpdate
  (params (LIves :type Integer))
  ;[1 1 1] Update Lives UI
  (Default|UpdateLives (Variables|Default|GetDisplayed_Lives) LIves))

(event Input|ActionEvents|InputActionInput-Positive
  (params (Key :type Key%20Structure :default "None"))
  ;[1 1 1] User Click to Spawn Ball
)

(fn ConstructionScript)

(fn BPIRequestNextLevel
  (return 0))

(fn BPIRetrievePersistentData
  (return 0 0))