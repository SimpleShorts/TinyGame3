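; BP_Pawn_Bat is the paddle pawn for a ball-and-bat game, moving along a spline and spawning balls.
; A timeline played, reversed or stopped by movement events maps its value to spline distance, setting the bat anchor's transform with sweep.
; SpawnBall sets the state to Active and binds ball destruction to a life-loss message on the player state.
; The lives-update handler only switches on state, with no respawn wired.
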(event Custom|Move%20Right
  (bind _spline (Variables|Default|GetSpline))
  ;[1 1 1] Bat Timeline Logic
  (bind _bat_position_along_spline (Timeline|Bat%20Timeline Play)
    (:Update
      (Transformation|SetWorldTransform (Variables|Default|GetBat%20Anchor) (Math|Transform|MakeTransform (.location (Spline|GetTransformatDistanceAlongSpline _spline (* (Spline|GetSplineLength _spline) _bat_position_along_spline) "World" false)) (.rotation (Spline|GetTransformatDistanceAlongSpline _spline (* (Spline|GetSplineLength _spline) _bat_position_along_spline) "World" false)) "1.000000,1.000000,1.000000") true false))))

(event Custom|Stop%20Moving
  (bind _spline (Variables|Default|GetSpline))
  ;[1 1 1] Bat Timeline Logic
  (bind _bat_position_along_spline (Timeline|Bat%20Timeline Stop)
    (:Update
      (Transformation|SetWorldTransform (Variables|Default|GetBat%20Anchor) (Math|Transform|MakeTransform (.location (Spline|GetTransformatDistanceAlongSpline _spline (* (Spline|GetSplineLength _spline) _bat_position_along_spline) "World" false)) (.rotation (Spline|GetTransformatDistanceAlongSpline _spline (* (Spline|GetSplineLength _spline) _bat_position_along_spline) "World" false)) "1.000000,1.000000,1.000000") true false))))

(event Custom|Move%20Left
  (bind _spline (Variables|Default|GetSpline))
  ;[1 1 1] Bat Timeline Logic
  (bind _bat_position_along_spline (Timeline|Bat%20Timeline Reverse)
    (:Update
      (Transformation|SetWorldTransform (Variables|Default|GetBat%20Anchor) (Math|Transform|MakeTransform (.location (Spline|GetTransformatDistanceAlongSpline _spline (* (Spline|GetSplineLength _spline) _bat_position_along_spline) "World" false)) (.rotation (Spline|GetTransformatDistanceAlongSpline _spline (* (Spline|GetSplineLength _spline) _bat_position_along_spline) "World" false)) "1.000000,1.000000,1.000000") true false))))

(event Custom|Reset%20Bat
  (bind _spline (Variables|Default|GetSpline))
  ;[1 1 1] Bat Timeline Logic
  (bind _bat_position_along_spline (Timeline|Bat%20Timeline SetNewTime)
    (:Update
      (Transformation|SetWorldTransform (Variables|Default|GetBat%20Anchor) (Math|Transform|MakeTransform (.location (Spline|GetTransformatDistanceAlongSpline _spline (* (Spline|GetSplineLength _spline) _bat_position_along_spline) "World" false)) (.rotation (Spline|GetTransformatDistanceAlongSpline _spline (* (Spline|GetSplineLength _spline) _bat_position_along_spline) "World" false)) "1.000000,1.000000,1.000000") true false))))

(event Custom|Spawn%20Ball
  ;[1 1 1] Spawn Ball
  (CallFunction|ChangeBatState "NewEnumerator1")
  (bind _returnvalue (Game|SpawnActorfromClass "/Game/Framework/BP_Ball.BP_Ball_C" (Transformation|GetWorldTransform (Variables|Default|GetArrow_Ball_Spawn_Boint)) "AlwaysSpawn" 0 0))
  (Game|BindEventtoOnDestroyed _returnvalue (delegate Custom|Allow%20Respawn)))

(event Custom|Set%20Play%20Rate
  (params (NewRate :type Float%20%28single-precision%29))
  (Components|Timeline|SetPlayRate (Variables|Default|GetBat%20Timeline) NewRate))

(event Custom|Lose%20Life
  (Class|BPIFramework|BPILivesUpdate(Message) (Game|GetPlayerState 0) -1))

(event Custom|Allow%20Respawn
  (params (DestroyedActor :type Actor%20Object%20Reference))
  ;[1 1 1] Spawn Ball
  (switch Utilities|FlowControl|Switch|SwitchonBP_Enum_BatState (Variables|Default|GetPawn%20State)
    (:NewEnumerator1
      (CallFunction|LoseLife))))

(event EventBeginPlay
  ;[1 1 1] Shart
  (CallFunction|ResetBat))

(event EventBPILivesUpdate
  (params (LIves :type Integer))
  (switch Utilities|FlowControl|Switch|SwitchonBP_Enum_BatState (Variables|Default|GetPawn%20State)))

(fn ConstructionScript)

(fn ChangeBatState
  (params (New%20State :type BP_Enum_BatState%20Enum :default "NewEnumerator0"))
  (if (Utilities|Enum|NotEqual(Enum) New%20State (Variables|Default|GetPawn%20State))
    (Variables|Default|SetPawn%20State New%20State)))