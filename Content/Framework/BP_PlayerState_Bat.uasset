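; BP_PlayerState_Bat is a player state that tracks the player's score and lives through Blueprint Interface events.
; Incoming points and life changes are added to the running totals, and the new values are sent to player controller 0 by interface messages.
; A lives update also messages the player pawn, unless the count falls below zero, in which case the TitleScreen level opens to end the game.
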(event EventBPILivesUpdate
  (params (LIves :type Integer))
  ;[1 1 1] Update Lives
  (bind _output_get (Variables|Default|SetCurrentLives (+ LIves (Variables|Default|GetCurrentLives))))
  (if (< _output_get 0)
    (Game|OpenLevel(byName) "TitleScreen")
    (else
      (Class|BPIFramework|BPILivesUpdate(Message) (Game|Player|GetPlayerPawn 0))
      (Class|BPIFramework|BPILivesUpdate(Message) (Game|GetPlayerController 0) _output_get))))

(event EventBPIScoreUpdate
  (params (Points :type Integer))
  ;[1 1 1] Update Score
  (bind _output_get (Variables|Default|SetCurrentScore (+ Points (Variables|Default|GetCurrentScore))))
  (Class|BPIFramework|BPIScoreUpdate(Message) (Game|GetPlayerController 0) _output_get))

(fn ConstructionScript)