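; Game mode for the end screen, which creates the UI_EndTitle widget on BeginPlay and adds it to the viewport.
; The BPI start-game event runs once, removing UITitleScreen (a variable never assigned here, unlike UIEndTitle) and opening Level1.
; The next-level and persistent-data interface functions are stubs returning zero values.
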(event EventBeginPlay
  (bind _returnvalue (UserInterface|CreateWidget "/Game/Framework/UI/UI_EndTitle.UI_EndTitle_C"))
  (bind _output_get (Variables|Default|SetUI_EndTitle _returnvalue))
  (UserInterface|Viewport|AddtoViewport _output_get 0))

(event EventBPIStartGame
  (Utilities|FlowControl|DoOnce false
    (:Completed
      (Widget|RemovefromParent (Variables|Default|GetUI_TitleScreen))
      (Game|OpenLevel(byName) "Level1"))))

(fn ConstructionScript)

(fn BPIRequestNextLevel
  (return 0))

(fn BPIRetrievePersistentData
  (return 0 0))