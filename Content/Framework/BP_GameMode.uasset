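; Game mode that handles level progression when it receives the level-complete interface event.
; It asks the Game Instance for the next level index and opens that entry in its level list by name, falling back to the title screen when the index runs past the end.
; Its own next-level and persistent-data interface functions only return zeroed defaults.
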(event EventBPILevelComplete
  (bind _arraylevellist (Variables|Default|GetarrayLevelList))
  (bind _updatedlevel (Class|BPIFramework|BPIRequestNextLevel(Message) (Game|GetGameInstance)))
  (if (< _updatedlevel (Utilities|Array|Length _arraylevellist))
    (Game|OpenLevel(byName) (Utilities|Array|Get(acopy) _arraylevellist _updatedlevel))
    (else
      (Game|OpenLevel(byName) "TitleScreen"))))

(fn ConstructionScript)

(fn BPIRequestNextLevel
  (return 0))

(fn BPIRetrievePersistentData
  (return 0 0))