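; Player controller that drives the player's bat pawn with mouse movement.
; On possess, it casts the pawn to BP_Pawn_Bat and stores the reference.
; The mouse axis is scaled by sensitivity, and its sign moves the bat right or left or stops it, with the scaled value also feeding the bat's play rate.
; A SpawnBall call is left unconnected, and BeginPlay only prints a test string.
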(event EventBeginPlay
  (Development|PrintString "test"))

(event EventPossess
  (params (PossessedPawn :type Pawn%20Object%20Reference))
  ;[1 1 1] On Possess
  (bind _asbp_pawn_bat (Utilities|Casting|CastToBP_Pawn_Bat PossessedPawn)
    (:then
      (Variables|Default|SetAs%20BP%20Pawn%20Bat _asbp_pawn_bat))
    (:CastFailed
      (Development|PrintString "Oh shart, didn't cast"))))

(event Input|AxisEvents|InputAxisMove-Mouse
  (params (AxisValue :type Float%20%28single-precision%29))
  (bind _as_bp_pawn_bat (Variables|Default|GetAs%20BP%20Pawn%20Bat))
  ;[1 1 1] Move Bat
  (bind _output_get (Variables|Default|SetMouse%20Move%20Rate (* AxisValue (Variables|Default|GetMouse%20Sensitvity))))
  (Math|Float|CompareFloat _output_get 0.0
    (:>
      (Default|MoveRight _as_bp_pawn_bat)
      (Default|SetPlayRate _as_bp_pawn_bat (Variables|Default|GetMouse%20Move%20Rate) :!label _label))
    (:==
      (Default|StopMoving _as_bp_pawn_bat))
    (:<
      (Default|MoveLeft _as_bp_pawn_bat)
      (Math|Float|NegateFloat (Variables|Default|GetMouse%20Move%20Rate)
        (:%20%20
          (goto _label))))))

(fn ConstructionScript)