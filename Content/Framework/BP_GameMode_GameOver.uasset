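; Game mode for the game over screen, which creates the game over widget and adds it to the viewport on BeginPlay.
; Its interface functions are stubs: start game does nothing, and the next level and persistent data requests return zeros.
; An unconnected DoOnce chain that would remove a title screen widget and open Level1 never runs.
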(event EventBeginPlay
  (bind _returnvalue (UserInterface|CreateWidget "/Game/Framework/UI/UI_GameOver.UI_GameOver_C"))
  (bind _output_get (Variables|Default|SetUI_GameOver _returnvalue))
  (UserInterface|Viewport|AddtoViewport _output_get 0))

(event EventBPIStartGame)

(fn ConstructionScript)

(fn BPIRequestNextLevel
  (return 0))

(fn BPIRetrievePersistentData
  (return 0 0))