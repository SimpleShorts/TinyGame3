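; BP_Brick2 is a destructible brick actor that awards points when the ball hits it.
; The BPIBallImpact interface event fires once, sending the points value and a brick-destroyed message to the player state through interface calls.
; It then applies a kinematic field to its Geometry Collection and, after a brief delay, spawns an actor at a randomly jittered offset from the brick, followed by a debug print.
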(event EventBPIBallImpact
  (bind _returnvalue (Game|GetPlayerState 0))
  (bind _brick_geometrycollection1 (Variables|Default|GetBrick_GeometryCollection1))
  (bind _randomtransformoffset (Variables|Default|GetRandomTransformOffset))
  (bind _returnvalue_2 (Transformation|GetWorldTransform _brick_geometrycollection1))
  (bind _returnvalue_3 (/ _randomtransformoffset 2))
  ;[1 1 1] Impact detector and score update
  (Utilities|FlowControl|DoOnce false
    (:Completed
      (Class|BPIFramework|BPIScoreUpdate(Message) _returnvalue (Variables|Default|GetPointsValue))
      ;[1 1 1] Brick Destruction Physics
      (Class|BPIFramework|BPIBrickDestroyed(Message) _returnvalue)
      (Class|GeometryCollectionComponent|ApplyKinematicField (Variables|Default|GetBrick_GeometryCollection1) 5e+03 "0, 0, 0")
      (Utilities|FlowControl|Delay 0.02)
      (Game|SpawnActorfromClass (Variables|Default|GetClass) (Math|Transform|MakeTransform (Math|Vector|MakeVector (+ (.x (.location _returnvalue_2)) (- (* (Math|Random|RandomFloat) _randomtransformoffset) _returnvalue_3)) (+ (.y (.location _returnvalue_2)) (Math|Float|MakeLiteralFloat 3e+01)) (+ (.z (.location _returnvalue_2)) (Utilities|Operators|Subtract (* (Math|Random|RandomFloat) _randomtransformoffset) _returnvalue_3 3e+01))) (.rotation _returnvalue_2) (.scale _returnvalue_2)) "AlwaysSpawn" 0 0)
      (Development|PrintString "well, we tried."))))

(fn ConstructionScript)