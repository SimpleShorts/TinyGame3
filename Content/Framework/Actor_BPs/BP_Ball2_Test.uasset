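; BP_Ball2_Test is a projectile ball actor, apparently a test variant, that destroys itself on entering a clear zone.
; On hit it messages the other actor through an interface, then after a brief delay spawns a larger field system at the impact point.
; If vertical speed is within a small threshold, it deflects by swapping X and Z velocity components with random boosts, countering excessive horizontal movement.
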(event EventBPIClearZoneEntered
  (Utilities|FlowControl|DoOnce false
    (:Completed
      (Actor|DestroyActor))))

(event Collision|EventHit
  (params (MyComp :type Primitive%20Component%20Object%20Reference) (Other :type Actor%20Object%20Reference) (OtherComp :type Primitive%20Component%20Object%20Reference) (bSelfMoved :type Boolean) (HitLocation :type Vector :default "0, 0, 0") (HitNormal :type Vector :default "0, 0, 0") (NormalImpulse :type Vector :default "0, 0, 0") (Hit :type Hit%20Result%20Structure%20%28by%20ref%29))
  (bind _returnvalue (Math|Random|RandomFloat))
  (bind _vertical_movement_trigger (Variables|Default|Getvertical_movement_trigger))
  (bind _deflect_randomizer (Variables|Default|Getdeflect_randomizer))
  (bind _projectilemovement (Variables|Default|GetProjectileMovement))
  (bind _returnvalue_2 (* _returnvalue _deflect_randomizer))
  (bind _updatedprimitive (Variables|/Script/Engine.MovementComponent|GetUpdatedPrimitive _projectilemovement))
  (bind _returnvalue_3 (Transformation|GetComponentVelocity _updatedprimitive))
  (bind (_x _y _z) (Math|Vector|BreakVector _returnvalue_3))
  (Class|BPIBall|BPIBallImpact(Message) Other)
  (Utilities|FlowControl|Delay 0.04)
  (Game|SpawnActorfromClass "/Game/Destruction/BP_FieldSystem2_Larger.BP_FieldSystem2_Larger_C" (Math|Transform|MakeTransform HitLocation "0, 0, 0" "1.000000,1.000000,1.000000") "AlwaysSpawn" 0 0)
  ;[1 1 1] Excessive horizontal movement detector
  (if (Math|Float|InRange(Float) _z (* _vertical_movement_trigger -1.0) _vertical_movement_trigger)
    (if (> _z 0.0)
      (Variables|Default|SetZ_velocity (+ _z _returnvalue_2))
      (else
        (Variables|Default|SetZ_velocity (- _z _returnvalue_2))))
    (Game|Components|ProjectileMovement|SetVelocityinLocalSpace (Variables|Default|GetProjectileMovement) (Math|Vector|MakeVector (Variables|Default|GetZ_velocity) 0.0 (+ (Math|Float|Absolute(Float) _x) _returnvalue_2)))))

(fn ConstructionScript)