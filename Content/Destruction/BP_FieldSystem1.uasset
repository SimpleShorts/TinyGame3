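; BP_FieldSystem1 is a Chaos field actor that fires a one-shot radial destruction burst on BeginPlay.
; A radial falloff field, sized and centered on its sphere collision with no falloff, applies external cluster strain to break geometry.
; A radial vector with randomly scaled magnitude then applies linear velocity from the center, using the same falloff as a culling field to exclude anything outside the sphere.
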(event EventBeginPlay
  (bind _fieldsystemcomponent (Variables|Field|GetFieldSystemComponent))
  (bind _spherecollision (Variables|Default|GetSphereCollision))
  (bind _radialfallofffieldmagnitude (Variables|Default|GetRadialFalloffFieldMagnitude))
  (bind _radialfalloff (Variables|Default|GetRadialFalloff))
  (bind _returnvalue (Transformation|GetWorldLocation _spherecollision))
  (bind _returnvalue_2 (Components|Sphere|GetScaledSphereRadius _spherecollision))
  (bind _returnvalue_3 (Field|SetRadialFalloff _radialfalloff _radialfallofffieldmagnitude 0.0 1.0 0.0 _returnvalue_2 _returnvalue "Field_FallOff_None"))
  (Class|FieldSystemComponent|ApplyPhysicsField _fieldsystemcomponent true "Field_ExternalClusterStrain" 0 _returnvalue_3)
  (Class|FieldSystemComponent|ApplyPhysicsField _fieldsystemcomponent true "Field_LinearVelocity" 0 (Field|SetCullingField (Variables|Default|GetCullingField) _returnvalue_3 (Field|SetRadialVector (Variables|Default|GetRadialVector) (* (Variables|Default|GetRadialVectorFieldMagnitude) (Math|Random|RandomFloatinRange 2.0 8.0)) _returnvalue) "Field_Culling_Outside")))

(fn ConstructionScript)